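; Openable door actor that swings open and closed on yaw in response to its OpenDoor OnOpen and OnClose events.
; BeginPlay caches the initial rotation, and a timeline combines its OpenAngle with that rotation, playing forward to open and in reverse to close.
; A timeline event plays the Doorlock sound at PlayerLocation, whose only assignment is in unconnected nodes that never run.
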(event OnOpen(OpenDoor)
  (bind _open_angle (Timeline|Timeline_0 Play)
    (:Update
      (Transformation|SetActorRotation (Math|Rotator|CombineRotators (Math|Rotator|MakeRotator 0.0 0.0 _open_angle) (Variables|Default|GetinitialRotation))))
    (:Sound%20Timing
      (Audio|PlaySoundatLocation "/Game/Audio/door-lock.door-lock" (stale _output_get)))))

(event OnClose(OpenDoor)
  (bind _open_angle (Timeline|Timeline_0 Reverse)
    (:Update
      (Transformation|SetActorRotation (Math|Rotator|CombineRotators (Math|Rotator|MakeRotator 0.0 0.0 _open_angle) (Variables|Default|GetinitialRotation))))
    (:Sound%20Timing
      (Audio|PlaySoundatLocation "/Game/Audio/door-lock.door-lock" (stale _output_get)))))

(event EventBeginPlay
  (Variables|Default|SetinitialRotation (Transformation|GetActorRotation)))

(fn ConstructionScript)